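; Melee weapon actor that supplies its wielder with attack montages, damage level, hit sound and socket transforms.
; Attack montages cycle by attack count through regular or combo arrays; charge uses one fixed montage.
; Toggles drive a blade glimmer material, blood particles that spawn decals on collision, and a brief animated trail in two variants.
; Dropping the weapon switches its mesh to simulated physics.
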(event OnParticleCollide(PBlood)
  (params (EventName :type Name :default "None") (EmitterTime :type Float%20%28single-precision%29) (ParticleTime :type Integer) (Location :type Vector :default "0, 0, 0") (Velocity :type Vector :default "0, 0, 0") (Direction :type Vector :default "0, 0, 0") (Normal :type Vector :default "0, 0, 0") (BoneName :type Name :default "None") (PhysMat :type Physical%20Material%20Object%20Reference))
  (Rendering|Decal|SpawnDecalatLocation "/Game/Materials/M_Decal_Inst.M_Decal_Inst" "10.000000,10.000000,10.000000" Location "-90.000000,0.000000,0.000000" 0.0))

(event EventBeginPlay
  (bind _returnvalue (Rendering|Material|CreateDynamicMaterialInstance (Variables|Default|GetWeapon_Mesh) 0 "/Game/InfinityBladeWeapons/Weapons/Blade/Swords/Blade_Glimmer/M_Blade_Glimmer.M_Blade_Glimmer" "None" :!class /Script/Engine.PrimitiveComponent))
  (Variables|Default|Setweapon%20material _returnvalue))

(event Collision|EventActorBeginOverlap
  (params (OtherActor :type Actor%20Object%20Reference)))

(event EventTick
  (params (DeltaSeconds :type Float%20%28single-precision%29)))

(event EventToggleBloodTrail
  (params (enable :type Boolean))
  (bind _p_blood (Variables|Default|GetP%20Blood))
  (if enable
    (Components|Activation|Activate _p_blood true)
    (else
      (Components|Activation|Deactivate _p_blood))))

(event EventToggleWeaponTrail
  (params (enable :type Boolean) (TrailType :type Integer))
  (bind _trail (Variables|Default|GetTrail))
  (if enable
    (Components|Animation|PlayAnimation _trail (Utilities|Select :Index TrailType :Option%200 "/Game/Particles/SwordTrail/Cube/CubeAnim.CubeAnim" :Option%201 "/Game/Particles/SwordTrail/Cube/CubeAnim_Red.CubeAnim_Red") true)
    (Utilities|FlowControl|Delay 0.2)
    (Audio|Components|Audio|Stop _trail)))

(fn ConstructionScript)

(event EventDropWeapon
  (bind _weapon_mesh (Variables|Default|GetWeapon_Mesh))
  (Collision|SetCollisionEnabled _weapon_mesh "PhysicsOnly")
  (Collision|SetCollisionProfileName _weapon_mesh "BlockAll" true :!class /Script/Engine.PrimitiveComponent)
  (Physics|SetSimulatePhysics _weapon_mesh true))

(event EventToggleChargeWeaopon
  (params (enable :type Boolean))
  (Rendering|Material|SetScalarParameterValue (Variables|Default|Getweapon%20material) "Charge multiplier" (select enable 5e+01 0.0) :!class /Script/Engine.MaterialInstanceDynamic))

(fn GetAttackMontage
  (params (attack%20Count :type Integer) (IsComboAttack :type Boolean))
  (bind _regular_attacks (Variables|Default|Getregular%20attacks))
  (bind _combo_attacks (Variables|Default|GetCombo%20attacks))
  (if IsComboAttack
    (return (Utilities|Array|Get(acopy) _combo_attacks (Math|Integer|%(Integer) attack%20Count (Utilities|Array|Length _combo_attacks))))
    (else
      (return (Utilities|Array|Get(acopy) _regular_attacks (Math|Integer|%(Integer) attack%20Count (Utilities|Array|Length _regular_attacks)))))))

(fn GetChargeMontage
  (return "/Game/Character/Knight/Sword/Sword_And_Shield_Slash_Montage_Charge.Sword_And_Shield_Slash_Montage_Charge"))

(fn GetDamageLevel
  (return (Variables|Default|GetdamageLevel)))

(fn GetHitSound
  (return (Variables|Default|GetenemyHitSound)))

(fn GetWeaponSocketTransform
  (params (socket%20name :type Name :default "None"))
  (return (Transformation|GetSocketTransform (Variables|Default|GetWeapon_Mesh) socket%20name "RTS_World")))